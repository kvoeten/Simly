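; Pickup actor that can be grabbed, released, highlighted on overlap and pushed by gravity-direction changes.
; The construction script applies a static mesh, or else a skeletal mesh, with configurable scale, offset and rotation.
; Grab stops Box physics, attaches it to the given socket and clears the custom-depth outline; release detaches and restores physics.
; Gravity changes add the direction to the mesh's velocity, only while that mesh simulates physics.
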(event `self.ReceiveBeginPlay`)

(event `Change Gravity Direction`
  (params (Direction :type "Vector Structure"))
  (`self.ChangeGravity` Direction))

(event `self.Grab`
  (params (`Initiatior Object` :type "SceneComponent Object Reference") (Socket :type Name))
  (`PrimitiveComponent.SetSimulatePhysics` (`self.Box`) false)
  (`SceneComponent.K2_AttachToComponent` (`self.Box`) `Initiatior Object` Socket "KeepWorld" "KeepWorld" "KeepWorld" true)
  (`self.ExitOverlap`))

(event `self.Release`
  (`PrimitiveComponent.SetSimulatePhysics` (`self.Box`) true)
  (`self.K2_DetachFromActor` "KeepWorld" "KeepWorld" "KeepWorld"))

(event `self.EnterOverlap`
  (`self.ToggleOutline` true))

(event `self.ExitOverlap`
  (`self.ToggleOutline` false))

(fn `ChangeGravity`
  (params (Direction :type "Vector Structure"))
  (bind _mesh (`self.Mesh`))
  (bind _skeleton (`self.Skeleton`))
  (`/Engine/EditorBlueprintResources/StandardMacros.IsValid` _mesh
    (:`Is Valid`
      (if (`SceneComponent.IsSimulatingPhysics` _mesh "None")
        (bind _returnvalue (`PrimitiveComponent.GetPhysicsLinearVelocity` _mesh "None"))
        (`PrimitiveComponent.SetPhysicsLinearVelocity` _mesh (+ _returnvalue Direction) false "None")))
    (:`Is Not Valid`
      (`/Engine/EditorBlueprintResources/StandardMacros.IsValid` _skeleton
        (:`Is Valid`
          (if (`SceneComponent.IsSimulatingPhysics` _skeleton "None")
            (bind _returnvalue_2 (`PrimitiveComponent.GetPhysicsLinearVelocity` _skeleton "None"))
            (`PrimitiveComponent.SetPhysicsLinearVelocity` _skeleton (+ _returnvalue_2 Direction) false "None")))))))

(fn `SetRelativePosition`
  (bind _offset (`self.Offset`))
  (bind _offsetrotation (`self.OffsetRotation`))
  (bind _mesh (`self.Mesh`))
  (bind _skeleton (`self.Skeleton`))
  (bind _scale (`self.Scale`))
  (`/Engine/EditorBlueprintResources/StandardMacros.IsValid` (`self.StaticMesh`)
    (:`Is Valid`
      (`SceneComponent.SetRelativeScale3D` _mesh _scale)
      (`SceneComponent.K2_AddRelativeLocation` _mesh _offset false false)
      (`SceneComponent.K2_SetRelativeRotation` _mesh _offsetrotation false false))
    (:`Is Not Valid`
      (`/Engine/EditorBlueprintResources/StandardMacros.IsValid` (`self.SkeletalMesh`)
        (:`Is Valid`
          (`SceneComponent.SetRelativeScale3D` _skeleton _scale)
          (`SceneComponent.K2_AddRelativeLocation` _skeleton _offset false false)
          (`SceneComponent.K2_SetRelativeRotation` _skeleton _offsetrotation false false))))))

(fn `ToggleOutline`
  (params (Enable :type Boolean))
  (bind _mesh (`self.Mesh`))
  (bind _skeleton (`self.Skeleton`))
  (`/Engine/EditorBlueprintResources/StandardMacros.IsValid` _mesh
    (:`Is Valid`
      (`PrimitiveComponent.SetRenderCustomDepth` _mesh Enable))
    (:`Is Not Valid`
      (`/Engine/EditorBlueprintResources/StandardMacros.IsValid` _skeleton
        (:`Is Valid`
          (`PrimitiveComponent.SetRenderCustomDepth` _skeleton Enable))))))

(fn `UserConstructionScript`
  (bind _staticmesh (`self.StaticMesh`))
  (bind _skeletalmesh (`self.SkeletalMesh`))
  (`/Engine/EditorBlueprintResources/StandardMacros.IsValid` _staticmesh
    (:`Is Valid`
      (`StaticMeshComponent.SetStaticMesh` (`self.Mesh`) _staticmesh))
    (:`Is Not Valid`
      (`/Engine/EditorBlueprintResources/StandardMacros.IsValid` _skeletalmesh
        (:`Is Valid`
          (`SkinnedMeshComponent.SetSkinnedAssetAndUpdate` (`self.Skeleton`) _skeletalmesh true)))))
  (`self.SetRelativePosition`))